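; Interactive sliding barn gate that alternates between open and closed each time InteractCase fires.
; BeginPlay stores the gate mesh's relative location as closed, and a FlipFlop sets start and end points between it and a fixed X offset.
; The Gate_Movement timeline lerps the mesh between those points, with an IsMoving flag ignoring new interactions until it finishes.
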(event Collision|EventActorBeginOverlap
  (params (OtherActor :type Actor%20Object%20Reference))
  (|CallParentFunction OtherActor) ; This node is disabled and will not be called.\nDrag off pins to build functionality.
)

(event EventTick
  (params (DeltaSeconds :type Float%20%28single-precision%29))
  (|CallParentFunction DeltaSeconds) ; This node is disabled and will not be called.\nDrag off pins to build functionality.
)

(event EventInteractCase
  (bind _closedlocation (Variables|Default|GetClosedLocation))
  (bind _closedlocation_2 (Variables|Default|GetClosedLocation))
  (if (not (Variables|Default|GetIsMoving))
    (Variables|Default|SetIsMoving true)
    (Utilities|FlowControl|FlipFlop
      (:A
        (Variables|Default|SetCurrentStart _closedlocation)
        (Variables|Default|SetCurrentEnd (+ _closedlocation "410.000000,0.000000,0.000000"))
        (bind _alpha (Timeline|Gate_Movement PlayFromStart)
          (:Update
            (Transformation|SetRelativeLocation (Variables|Default|GetSM_Barn_Gates) (Math|Vector|Lerp(Vector) (Variables|Default|GetCurrentStart) (Variables|Default|GetCurrentEnd) _alpha) false false))
          (:Finished
            (Variables|Default|SetIsMoving false))))
      (:B
        (Variables|Default|SetCurrentStart (+ _closedlocation_2 "410.000000,0.000000,0.000000"))
        (Variables|Default|SetCurrentEnd _closedlocation_2)
        (Timeline|Gate_Movement PlayFromStart)))))

(event EventBeginPlay
  (Variables|Default|SetClosedLocation (Variables|/Script/Engine.SceneComponent|GetRelativeLocation (Variables|Default|GetSM_Barn_Gates))))

(fn ConstructionScript
  (|CallParentFunction))