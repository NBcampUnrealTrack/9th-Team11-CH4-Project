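; Player pawn blueprint that adds a camera-driven scan ability and plays a sound when grabbing an object succeeds.
; On BeginPlay it creates a dynamic scan post-process material and adds it as a blendable on the follow camera.
; Pressing scan runs a timeline that expands the ScanComponent's distance and feeds camera origin, forward, intensity and grid falloff to the material, then finishes the scan.
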(event EventBeginPlay
  (bind _returnvalue (Rendering|Material|CreateDynamicMaterialInstance "/Game/NoPhotos/Blueprints/Relic/Outline/Material/MI_PP_Scan.MI_PP_Scan" "None" "None" :!class /Script/Engine.KismetMaterialLibrary))
  (bind _output_get (Variables|Default|SetNewVar _returnvalue))
  (Rendering|AddorUpdateBlendable (Variables|Default|GetFollowCamera) _output_get 1.0 :!class /Script/Engine.CameraComponent))

(event Collision|EventActorBeginOverlap
  (params (OtherActor :type Actor%20Object%20Reference)))

(event EventTick
  (params (DeltaSeconds :type Float%20%28single-precision%29)))

(event EventOnGrabSucceeded
  (params (GrabbedComponent :type Primitive%20Component%20Object%20Reference))
  (Utilities|IsValid GrabbedComponent
    (:Is%20Valid
      (Class|NPSoundSubsystem|PlaySFX (Subsystems|GetNPSoundSubsystem) 0 1.0 1.0 0.0))))

(event EventEventPressScan
  (bind _newvar (Variables|Default|GetNewVar))
  (bind _newvar_2 (Variables|Default|GetNewVar))
  (bind _followcamera (Variables|Default|GetFollowCamera))
  (Class|NPScanComponent|StartScan (Variables|Default|GetScanComponent) (Variables|Default|GetScanDistance))
  (bind (_direction _distance _intensity _pow) (Timeline|Timeline PlayFromStart)
    (:Update
      (Class|NPScanComponent|UpdateScanDistance (Variables|Default|GetScanComponent) (* _distance (Variables|Default|GetScanDistance)))
      (Rendering|Material|SetScalarParameterValue _newvar_2 "ScanDistance" (* _distance (Variables|Default|GetScanDistance)) :!class /Script/Engine.MaterialInstanceDynamic)
      (Rendering|Material|SetVectorParameterValue _newvar_2 "ScanOrigin" (Math|Conversions|ToLinearColor(Vector) (Transformation|GetWorldLocation _followcamera)) :!class /Script/Engine.MaterialInstanceDynamic)
      (Rendering|Material|SetVectorParameterValue _newvar_2 "ScanForward" (Math|Conversions|ToLinearColor(Vector) (Math|Vector|GetForwardVector _followcamera)) :!class /Script/Engine.MaterialInstanceDynamic)
      (Rendering|Material|SetScalarParameterValue _newvar "ScanIntensity" (* _intensity 1.0) :!class /Script/Engine.MaterialInstanceDynamic)
      (Rendering|Material|SetScalarParameterValue _newvar "ScanGridPow" _pow :!class /Script/Engine.MaterialInstanceDynamic))
    (:Finished
      (Class|NPScanComponent|FinishScan (Variables|Default|GetScanComponent)))))

(fn ConstructionScript)