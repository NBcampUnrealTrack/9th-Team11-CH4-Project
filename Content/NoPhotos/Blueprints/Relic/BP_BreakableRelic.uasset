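; BP_BreakableRelic is a breakable relic Blueprint that adds sound feedback for damage and breaking.
; On each damage event it plays a hit sound through NPSoundSubsystem, mapping lost health to pitch between PitchMin and PitchMax.
; On breaking it plays a broken sound with slight random pitch variation.
; Both sounds play at the relic's location with shared attenuation, and the Blueprint contains no damage or health logic itself.
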(event EventBeginPlay)

(event Collision|EventActorBeginOverlap
  (params (OtherActor :type Actor%20Object%20Reference)))

(event EventTick
  (params (DeltaSeconds :type Float%20%28single-precision%29)))

(event EventOnRelicDamaged
  (params (Damage :type Integer) (CurrentHealth :type Integer) (MaxHealth :type Integer) (RemainingHealthRatio :type Float%20%28single-precision%29))
  ;[0.15 0.15 0.15 0.5] Hit Sound
  (Class|NPSoundSubsystem|PlaySFXatLocation (Subsystems|GetNPSoundSubsystem) (Variables|Default|GetHit%20Sound) (Transformation|GetActorLocation) "0, 0, 0" 1.0 (Math|Float|MapRangeClamped (- 1.0 RemainingHealthRatio) 0.0 1.0 (Variables|Default|GetPitchMin) (Variables|Default|GetPitchMax)) 0.0 "/Game/NoPhotos/Blueprints/Relic/GeometryCollections/ATT_Breakable.ATT_Breakable" 0))

(event EventOnRelicBroken
  ;[0.15 0.15 0.15 0.5] Broken Sound
  (Class|NPSoundSubsystem|PlaySFXatLocation (Subsystems|GetNPSoundSubsystem) (Variables|Default|GetBroken%20Sound) (Transformation|GetActorLocation) "0, 0, 0" 1.0 (Math|Float|MapRangeClamped (Math|Random|RandomFloat) 0.0 1.0 0.9 1.1) 0.0 "/Game/NoPhotos/Blueprints/Relic/GeometryCollections/ATT_Breakable.ATT_Breakable" 0))

(fn ConstructionScript)