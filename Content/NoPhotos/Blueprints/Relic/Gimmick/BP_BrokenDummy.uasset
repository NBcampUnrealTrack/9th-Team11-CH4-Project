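; Breakable dummy gimmick that reacts to hard physics hits, cracks in stages and shatters.
; Hits above an impulse threshold spawn wood particles, call the parent's OnExecute and play a pitch-randomized sound.
; NPPinata damage-stage events drive CrackAmount on a dynamic material instance.
; Its broken event swaps the static mesh for a Geometry Collection, crumbles it and applies a radial impulse at the impact point.
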(event OnPinataBroken(NPPinata)
  (params (ImpactLocation :type Vector :default "0, 0, 0"))
  (bind _staticmesh (Variables|Default|GetStaticMesh))
  (bind _geometrycollection (Variables|Default|GetGeometryCollection))
  (Development|PrintString "broken")
  (Development|SetHiddeninGame _staticmesh true false)
  (Collision|SetCollisionEnabled _staticmesh "NoCollision")
  (Development|SetHiddeninGame _geometrycollection false false)
  (Collision|SetCollisionEnabled _geometrycollection "QueryAndPhysics")
  (Physics|SetSimulatePhysics _geometrycollection true)
  (Class|GeometryCollectionComponent|CrumbleActiveClusters _geometrycollection)
  (Physics|AddRadialImpulse _geometrycollection ImpactLocation 2e+02 1e+03 "RIF_Linear" true))

(event OnComponentHit(StaticMesh)
  (params (HitComponent :type Primitive%20Component%20Object%20Reference) (OtherActor :type Actor%20Object%20Reference) (OtherComp :type Primitive%20Component%20Object%20Reference) (NormalImpulse :type Vector :default "0, 0, 0") (Hit :type Hit%20Result%20Structure%20%28by%20ref%29))
  (bind (_bblockinghit _binitialoverlap _time _distance _location _impactpoint _normal _impactnormal) (Collision|BreakHitResult Hit))
  (if (>= (Math|Vector|VectorLength NormalImpulse) 5e+03)
    (Effects|SpawnEmitteratLocation "/Game/Realistic_Starter_VFX_Pack_Vol2/Particles/Hit/P_Wood.P_Wood" _impactpoint (Math|Rotator|MakeRotfromZ _impactnormal))
    (|CallParentFunction 0 "")
    (Class|NPSoundSubsystem|PlaySFXatLocation (Subsystems|GetNPSoundSubsystem) "/Game/NoPhotos/Resources/Sound/SFX/Relic/S_Hit.S_Hit" (Transformation|GetActorLocation) "0, 0, 0" 1.0 (Math|Random|RandomFloatinRange 0.9 1.1) 0.0 "/Game/NoPhotos/Blueprints/Relic/GeometryCollections/ATT_Breakable.ATT_Breakable" 0)))

(event OnPinataDamageStageChanged(NPPinata)
  (params (DamageStage :type Integer))
  (bind _pinatamid (Variables|Default|GetPinataMID))
  (switch int DamageStage
    (:0
      (Rendering|Material|SetScalarParameterValue _pinatamid "CrackAmount" 0.0 :!class /Script/Engine.MaterialInstanceDynamic))
    (:1
      (Rendering|Material|SetScalarParameterValue _pinatamid "CrackAmount" 0.5 :!class /Script/Engine.MaterialInstanceDynamic))
    (:2
      (Rendering|Material|SetScalarParameterValue _pinatamid "CrackAmount" 1.0 :!class /Script/Engine.MaterialInstanceDynamic))))

(event EventBeginPlay
  (bind _returnvalue (Rendering|Material|CreateDynamicMaterialInstance (Variables|Default|GetStaticMesh) 0 "/Game/NoPhotos/Material/test/M_Universal_A.M_Universal_A" "None" :!class /Script/Engine.PrimitiveComponent))
  (bind _output_get (Variables|Default|SetPinataMID _returnvalue))
  (Rendering|Material|SetScalarParameterValue _output_get "CrackAmount" 0.0 :!class /Script/Engine.MaterialInstanceDynamic))

(event Collision|EventActorBeginOverlap
  (params (OtherActor :type Actor%20Object%20Reference)))

(event EventTick
  (params (DeltaSeconds :type Float%20%28single-precision%29)))

(fn ConstructionScript)