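; BP_MammothLegGimmik is a relic gimmick, apparently a mammoth leg, that responds to successful pulls counted against a required total.
; Each successful pull plays a bone-break sound at the actor's location with slightly randomized pitch and nearby attenuation.
; When the required pull count is reached, it also disables actor collision and activates the BurstMiniImpact effect.
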(event OnPullSucceeded(NPPullGimmick)
  (params (CurrentPullCount :type Integer) (RequiredPullCount :type Integer))
  (if (>= CurrentPullCount RequiredPullCount)
    (Collision|SetActorEnableCollision false)
    (CallFunction|PlaySound)
    (Components|Activation|SetActive (Variables|Default|GetBurst_Mini_Impact) true true)
    (else
      (CallFunction|PlaySound))))

(event Custom|PlaySound
  (Class|NPSoundSubsystem|PlaySFXatLocation (Subsystems|GetNPSoundSubsystem) "/Game/NoPhotos/Resources/Sound/SFX/Relic/S_Bone_Break.S_Bone_Break" (Transformation|GetActorLocation) "0, 0, 0" 1.0 (Math|Random|RandomFloatinRange 0.9 1.1) 0.0 "/Game/NoPhotos/Blueprints/Relic/GeometryCollections/ATT_Nearby.ATT_Nearby" 0))

(event EventBeginPlay)

(event Collision|EventActorBeginOverlap
  (params (OtherActor :type Actor%20Object%20Reference)))

(event EventTick
  (params (DeltaSeconds :type Float%20%28single-precision%29)))

(fn ConstructionScript)