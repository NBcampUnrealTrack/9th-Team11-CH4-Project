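; Base Blueprint for a relic display case that reacts to damage, breaking, locking and unlocking.
; Damage plays a glass-hit sound that grows louder as remaining health drops, and breaking plays a shatter sound and prints a debug message.
; Unlocking plays the Open timeline to move CollectionRoot vertically, scaled by Height, and locking reverses it.
; Both lock transitions are skipped once ImpactReceiveComponent reports the case broken.
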(event EventBeginPlay)

(event Collision|EventActorBeginOverlap
  (params (OtherActor :type Actor%20Object%20Reference)))

(event EventTick
  (params (DeltaSeconds :type Float%20%28single-precision%29)))

(event EventOnCaseDamaged
  (params (RemainingHealthRatio :type Float%20%28single-precision%29))
  (Class|NPSoundSubsystem|PlaySFXatLocation (Subsystems|GetNPSoundSubsystem) "/Game/NoPhotos/Resources/Sound/SoundEffect/Relic/GlassHit.GlassHit" "0, 0, 0" "0, 0, 0" (+ (- 1.0 RemainingHealthRatio) 1.0) 1.0 0.0 0 0))

(event EventOnCaseBroken
  ;[0.15 0.15 0.15 0.5] Comment
  (Class|NPSoundSubsystem|PlaySFXatLocation (Subsystems|GetNPSoundSubsystem) "/Game/NoPhotos/Resources/Sound/SoundEffect/Relic/GlassBroken.GlassBroken" (Transformation|GetActorLocation) "0, 0, 0" 1.0 1.0 0.0 0 0)
  (Development|PrintString "케이스 박살"))

(event EventOnCaseUnlocked
  (if (not (Class|NPImpactReceiveComponent|IsBroken (Variables|Default|GetImpactReceiveComponent)))
    (bind _height (Timeline|Open Play)
      (:Update
        (Transformation|SetRelativeLocation (Variables|Default|GetCollectionRoot) (Math|Vector|MakeVector 0.0 0.0 (* _height (Variables|Default|GetHeight))) false false)))))

(event EventOnCaseLocked
  (if (not (Class|NPImpactReceiveComponent|IsBroken (Variables|Default|GetImpactReceiveComponent)))
    (bind _height (Timeline|Open Reverse)
      (:Update
        (Transformation|SetRelativeLocation (Variables|Default|GetCollectionRoot) (Math|Vector|MakeVector 0.0 0.0 (* _height (Variables|Default|GetHeight))) false false)))))

(fn ConstructionScript)