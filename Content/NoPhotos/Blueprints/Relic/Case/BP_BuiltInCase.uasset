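; BP_BuiltInCase is a built-in relic case that can be unlocked open or damaged and broken.
; Damage and break events play glass sounds at the case, with pitch driven by lost health for hits and randomized for breaking.
; Unless its ImpactReceiveComponent is broken, unlocking plays a timeline that swings the left and right scene components apart by OpenAngle, and locking reverses it.
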(event EventBeginPlay)

(event Collision|EventActorBeginOverlap
  (params (OtherActor :type Actor%20Object%20Reference)))

(event EventTick
  (params (DeltaSeconds :type Float%20%28single-precision%29)))

(event EventOnCaseDamaged
  (params (RemainingHealthRatio :type Float%20%28single-precision%29))
  (Class|NPSoundSubsystem|PlaySFXatLocation (Subsystems|GetNPSoundSubsystem) "/Game/NoPhotos/Resources/Sound/SFX/Relic/GlassHit.GlassHit" (Transformation|GetActorLocation) "0, 0, 0" 1.0 (Math|Float|MapRangeClamped (- 1.0 RemainingHealthRatio) 0.0 1.0 0.8 1.2) 0.0 "/Game/NoPhotos/Blueprints/Relic/GeometryCollections/ATT_Breakable.ATT_Breakable" 0))

(event EventOnCaseBroken
  ;[0.15 0.15 0.15 0.5] Comment
  (Class|NPSoundSubsystem|PlaySFXatLocation (Subsystems|GetNPSoundSubsystem) "/Game/NoPhotos/Resources/Sound/SFX/Relic/GlassBroken.GlassBroken" (Transformation|GetActorLocation) "0, 0, 0" 1.0 (Math|Float|MapRangeClamped (Math|Random|RandomFloat) 0.0 1.0 0.9 1.1) 0.0 "/Game/NoPhotos/Blueprints/Relic/GeometryCollections/ATT_Breakable.ATT_Breakable" 0)
  (Development|PrintString "케이스 박살"))

(event EventOnCaseUnlocked
  (if (not (Class|NPImpactReceiveComponent|IsBroken (Variables|Default|GetImpactReceiveComponent)))
    (Development|PrintString "Built in Unlocked")
    (bind _angle (Timeline|Open Play)
      (:Update
        (Transformation|SetRelativeRotation (Variables|Default|GetSceneR) (Math|Rotator|MakeRotator 0.0 0.0 (* (Variables|Default|GetOpenAngle) _angle)) false false)
        (Transformation|SetRelativeRotation (Variables|Default|GetSceneL) (Math|Rotator|MakeRotator 0.0 0.0 (* (Variables|Default|GetOpenAngle) -1.0 _angle)) false false)))))

(event EventOnCaseLocked
  (if (not (Class|NPImpactReceiveComponent|IsBroken (Variables|Default|GetImpactReceiveComponent)))
    (bind _angle (Timeline|Open Reverse)
      (:Update
        (Transformation|SetRelativeRotation (Variables|Default|GetSceneR) (Math|Rotator|MakeRotator 0.0 0.0 (* (Variables|Default|GetOpenAngle) _angle)) false false)
        (Transformation|SetRelativeRotation (Variables|Default|GetSceneL) (Math|Rotator|MakeRotator 0.0 0.0 (* (Variables|Default|GetOpenAngle) -1.0 _angle)) false false)))))

(fn ConstructionScript)