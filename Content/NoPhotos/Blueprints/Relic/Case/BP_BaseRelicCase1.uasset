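; Base relic display case that plays sound and motion feedback as it is damaged, broken, locked or unlocked.
; While ImpactReceiveComponent reports the case unbroken, unlocking plays an Open timeline that moves CollectionRoot vertically by a height factor, and locking reverses it.
; Glass-hit volume rises as remaining health falls.
; Break, open and close sounds play at the actor's location with nearby attenuation through the NP sound subsystem.
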(event EventBeginPlay)

(event Collision|EventActorBeginOverlap
  (params (OtherActor :type Actor%20Object%20Reference)))

(event EventTick
  (params (DeltaSeconds :type Float%20%28single-precision%29)))

(event EventOnCaseDamaged
  (params (RemainingHealthRatio :type Float%20%28single-precision%29))
  (Class|NPSoundSubsystem|PlaySFXatLocation (Subsystems|GetNPSoundSubsystem) "/Game/NoPhotos/Resources/Sound/SFX/Relic/Case/GlassHit.GlassHit" "0, 0, 0" "0, 0, 0" (+ (- 1.0 RemainingHealthRatio) 1.0) 1.0 0.0 0 0))

(event EventOnCaseBroken
  ;[0.15 0.15 0.15 0.5] Comment
  (CallFunction|Play3DSound "/Game/NoPhotos/Resources/Sound/SFX/Relic/Case/GlassBroken.GlassBroken"))

(event EventOnCaseUnlocked
  (if (not (Class|NPImpactReceiveComponent|IsBroken (Variables|Default|GetImpactReceiveComponent)))
    (CallFunction|Play3DSound "/Game/NoPhotos/Resources/Sound/SFX/Relic/Case/S_CaseOpen.S_CaseOpen")
    (bind _height (Timeline|Open Play)
      (:Update
        (Transformation|SetRelativeLocation (Variables|Default|GetCollectionRoot) (Math|Vector|MakeVector 0.0 0.0 (* _height (Variables|Default|GetHeight))) false false)))))

(event EventOnCaseLocked
  (if (not (Class|NPImpactReceiveComponent|IsBroken (Variables|Default|GetImpactReceiveComponent)))
    (CallFunction|Play3DSound "/Game/NoPhotos/Resources/Sound/SFX/Relic/Case/S_CaseClose.S_CaseClose")
    (bind _height (Timeline|Open Reverse)
      (:Update
        (Transformation|SetRelativeLocation (Variables|Default|GetCollectionRoot) (Math|Vector|MakeVector 0.0 0.0 (* _height (Variables|Default|GetHeight))) false false)))))

(fn ConstructionScript)

(fn Play3DSound
  (params (Sound :type Sound%20Base%20Object%20Reference))
  (Class|NPSoundSubsystem|PlaySFXatLocation (Subsystems|GetNPSoundSubsystem) Sound (Transformation|GetActorLocation) "0, 0, 0" 1.0 1.0 0.0 "/Game/NoPhotos/Blueprints/Relic/GeometryCollections/ATT_Nearby.ATT_Nearby" 0))