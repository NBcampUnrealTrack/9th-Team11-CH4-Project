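; BP_PiratesHeart is the Pirate's Heart relic object, which fades in visually when it begins play.
; After running the parent's BeginPlay, it creates a dynamic material instance on the first slot of RelicMesh.
; The FadeIn timeline then drives that material's FadeAlpha parameter.
; The construction script only calls the parent.
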(event EventBeginPlay
  (|CallParentFunction)
  (bind _returnvalue (Rendering|Material|CreateDynamicMaterialInstance (Variables|Default|GetRelicMesh) 0 0 "None" :!class /Script/Engine.PrimitiveComponent))
  (bind _output_get (Variables|Default|SetFadeMaterial _returnvalue))
  (Rendering|Material|SetMaterial (Variables|Default|GetRelicMesh) 0 _output_get)
  (bind _alpha (Timeline|FadeIn Play)
    (:Update
      (Rendering|Material|SetScalarParameterValue (Variables|Default|GetFadeMaterial) "FadeAlpha" _alpha :!class /Script/Engine.MaterialInstanceDynamic))))

(fn ConstructionScript
  (|CallParentFunction))