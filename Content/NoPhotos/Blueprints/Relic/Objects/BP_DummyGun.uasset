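; Dummy gun relic object that plays a brief spark effect when used, with no projectile or damage logic of its own.
; It enables input for a player controller on BeginPlay and listens for the IA_RelicUse action.
; Each use waits briefly, attaches a spark emitter to RelicMesh, then destroys it shortly after.
; A DoOnce blocks repeat uses and resets only once that still-valid emitter is destroyed.
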(event Input|EnhancedActionEvents|EnhancedInputActionIA_RelicUse
  (params (ActionValue :type Boolean) (ElapsedSeconds :type Float%20%28double-precision%29) (TriggeredSeconds :type Float%20%28double-precision%29) (InputAction :type Input%20Action%20Object%20Reference :default "/Game/Input/Actions/IA_RelicUse.IA_RelicUse"))
  (:Started
    (Utilities|FlowControl|DoOnce false :!label _label
      (:Completed
        (Utilities|FlowControl|Delay 0.75)
        (bind _returnvalue (Effects|SpawnEmitterAttached "/Game/Realistic_Starter_VFX_Pack_Vol2/Particles/Sparks/P_Sparks_E.P_Sparks_E" (Variables|Default|GetRelicMesh) "None" "0, 0, 0" "0, 0, 0" "1.000000,1.000000,1.000000" "SnapToTarget"))
        (bind _output_get (Variables|Default|SetNewVar _returnvalue))
        (Utilities|FlowControl|Delay 0.2)
        (Utilities|IsValid _output_get
          (:Is%20Valid
            (Components|DestroyComponent _output_get)
            (goto _label Reset)))))))

(event EventBeginPlay
  (bind _returnvalue (Class|InputDeviceLibrary|GetPlayerControllerfromPlatformUser))
  (Input|EnableInput _returnvalue))

(event Collision|EventActorBeginOverlap
  (params (OtherActor :type Actor%20Object%20Reference))
  (|CallParentFunction OtherActor) ; This node is disabled and will not be called.\nDrag off pins to build functionality.
)

(event EventTick
  (params (DeltaSeconds :type Float%20%28single-precision%29))
  (|CallParentFunction DeltaSeconds) ; This node is disabled and will not be called.\nDrag off pins to build functionality.
)

(fn ConstructionScript
  (|CallParentFunction))