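; BP_ShipWheel is a ship wheel gimmick that activates once the wheel is turned far enough.
; While the wheel is grabbed, a looping timer polls the physics constraint's twist, and releasing it clears the timer.
; When the absolute twist reaches a quarter turn, it latches as activated, stops polling and sends the ship gimmick activation notification.
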(event Custom|CheckWheelRotation
  ;[0.15 0.15 0.15 0.5] 기믹 처리유무 확인
  (if (not (Variables|Default|GetIsWheelActivated))
    (if (>= (Math|Float|Absolute(Float) (Class|PhysicsConstraintComponent|GetCurrentTwist (Variables|Default|GetPhysicsConstraint))) 9e+01)
      (Variables|Default|SetIsWheelActivated true)
      (Utilities|Time|ClearandInvalidateTimerbyHandle (Variables|Default|GetWheelCheckTimer))
      (Class|NPShipGimmickBase|NotifyShipGimmickActivated))))

(event EventGrabStateChanged
  (params (bIsGrabbed :type Boolean))
  ;[0.15 0.15 0.15 0.5] 기믹 처리유무 확인
  (if bIsGrabbed
    (Utilities|Time|SetTimerbyEvent (delegate Custom|CheckWheelRotation) 0.05 true)
    (else
      (Utilities|Time|ClearandInvalidateTimerbyHandle (Variables|Default|GetWheelCheckTimer)))))

(fn ConstructionScript
  (|CallParentFunction))