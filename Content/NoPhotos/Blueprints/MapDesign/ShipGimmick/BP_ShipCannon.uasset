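; BP_ShipCannon is a ship gimmick: a cannon that fires when the player pulls a grabbable rope.
; BeginPlay attaches the rope's end to the gimmick mesh, and grabbing starts a short delay before recording that mesh's position.
; A looping timer, cleared on release, then measures displacement from that start point.
; Past a distance threshold it marks the cannon fired, stops the timer, plays an explosion sound and notifies that the gimmick activated.
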(event Custom|CheckCannonPull
  ;[0.15 0.15 0.15 0.5] 기믹 처리유무 확인
  (if (Variables|Default|GetIsCannonFired)
    _
    (else
      _))
  (if (>= (Math|Float|Absolute(Float) (Math|Vector|Distance(Vector) (Transformation|GetWorldLocation (Variables|Default|GetGimmickMesh)) (Variables|Default|GetPullStartLocation))) 1.2e+02)
    (Variables|Default|SetIsCannonFired true)
    (Utilities|Time|ClearandInvalidateTimerbyHandle (Variables|Default|GetCannonCheckTimer))
    (Audio|PlaySoundatLocation "/Game/NoPhotos/Resources/Sound/SFX/Relic/soundreality-explosion-fx-343683.soundreality-explosion-fx-343683" (Transformation|GetWorldLocation (Variables|Default|GetCannonMesh)) "0, 0, 0" 0.6 1.0 0.0 0 0 0 0)
    (Class|NPShipGimmickBase|NotifyShipGimmickActivated)))

(event EventGrabStateChanged
  (params (bIsGrabbed :type Boolean))
  ;[0.15 0.15 0.15 0.5] 기믹 처리유무 확인
  (Variables|Default|SetIsPulling bIsGrabbed)
  (if bIsGrabbed
    (Utilities|FlowControl|Delay 0.2)
    (if true
      (Variables|Default|SetPullStartLocation (Transformation|GetWorldLocation (Variables|Default|GetGimmickMesh)))
      (bind _returnvalue (Utilities|Time|SetTimerbyEvent (delegate Custom|CheckCannonPull) 0.05 true))
      (Variables|Default|SetCannonCheckTimer _returnvalue))
    (else
      (Utilities|Time|ClearandInvalidateTimerbyHandle (Variables|Default|GetCannonCheckTimer)))))

(event EventBeginPlay
  ;[0.15 0.15 0.15 0.5] 기믹 처리유무 확인
  (Class|CableComponent|SetAttachEndtoComponent (Variables|Default|GetPullRope) (Variables|Default|GetGimmickMesh) "None"))

(fn ConstructionScript)