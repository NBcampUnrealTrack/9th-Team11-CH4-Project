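; Ship gimmick anchor that counts as activated once it is placed at a snap transform.
; BeginPlay stores the mesh transform, breaks the physics constraint and strings the rope from RopeStart to the mesh.
; Grab changes toggle the AnchorZone target visual; the first placement stops physics, snaps the mesh and notifies gimmick activation.
; Reset clears the placed flag and applies the saved transform to the actor.
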(event Custom|PlaceAnchor
  (params (SnapTransform :type Transform))
  (bind _gimmickmesh (Variables|Default|GetGimmickMesh))
  ;[0.15 0.15 0.15 0.5] 기믹 처리여부 확인
  (if (not (Variables|Default|GetIsAnchorPlaced))
    (Variables|Default|SetIsAnchorPlaced true)
    (Physics|SetSimulatePhysics _gimmickmesh false)
    (Transformation|SetWorldTransform _gimmickmesh SnapTransform false false)
    (Class|NPShipGimmickBase|NotifyShipGimmickActivated)))

(event EventShipGimmickReset
  ;[0.15 0.15 0.15 0.5] 진행도 초기화
  (Variables|Default|SetIsAnchorPlaced false)
  (Transformation|SetActorTransform (Variables|Default|GetInitialTransform)))

(event EventGrabStateChanged
  (params (bIsGrabbed :type Boolean))
  (bind _anchorzone (Variables|Default|GetAnchorZone))
  ;[0.15 0.15 0.15 0.5] 기믹 처리여부 확인
  (Utilities|IsValid _anchorzone
    (:Is%20Valid
      (Default|SetTargetVisualVisible _anchorzone bIsGrabbed))))

(event EventBeginPlay
  ;[0.15 0.15 0.15 0.5] 바닥에 꽂기
  (Variables|Default|SetInitialTransform (Transformation|GetWorldTransform (Variables|Default|GetGimmickMesh)))
  (Class|PhysicsConstraintComponent|BreakConstraint (Variables|Default|GetPhysicsConstraint))
  (Utilities|IsValid (Variables|Default|GetRopeStart)
    (:Is%20Valid
      (Transformation|AttachComponentToComponent (Variables|Default|GetAnchorRope) (Variables|/Script/Engine.Actor|GetRootComponent (Variables|Default|GetRopeStart)) "None" "SnapToTarget" "SnapToTarget" "KeepRelative" false)
      (Class|CableComponent|SetAttachEndtoComponent (Variables|Default|GetAnchorRope) (Variables|Default|GetGimmickMesh) "None"))))

(fn ConstructionScript)