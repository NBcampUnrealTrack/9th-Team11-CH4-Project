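; BP_ShipBook is a ship book map gimmick that shows a ship info widget to a nearby player.
; Begin and end overlap show and hide the widget component, reacting only to a locally controlled NPReplicatedStablePhysicsPawn, so other players' pawns do not toggle it on that machine.
; Tick rotates the widget to face the first player's camera.
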(event Collision|EventActorBeginOverlap
  (params (OtherActor :type Actor%20Object%20Reference))
  (bind _asnpreplicated_stable_physics_pawn (Utilities|Casting|CastToNPReplicatedStablePhysicsPawn OtherActor))
  (if (Pawn|IsLocallyControlled _asnpreplicated_stable_physics_pawn)
    (Rendering|SetVisibility (Variables|Default|GetWC_ShipInfoComponent) true false)))

(event Collision|EventActorEndOverlap
  (params (OtherActor :type Actor%20Object%20Reference))
  (bind _asnpreplicated_stable_physics_pawn (Utilities|Casting|CastToNPReplicatedStablePhysicsPawn OtherActor))
  (if (Pawn|IsLocallyControlled _asnpreplicated_stable_physics_pawn)
    (Rendering|SetVisibility (Variables|Default|GetWC_ShipInfoComponent) false false)))

(event EventTick
  (params (DeltaSeconds :type Float%20%28single-precision%29))
  (bind _wc_shipinfocomponent (Variables|Default|GetWC_ShipInfoComponent))
  (Transformation|SetWorldRotation _wc_shipinfocomponent (Math|Rotator|FindLookatRotation (Transformation|GetWorldLocation _wc_shipinfocomponent) (Camera|GetCameraLocation (Game|GetPlayerCameraManager 0))) false false))

(fn ConstructionScript)