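; BP_CubeTrack is a map gimmick actor that procedurally builds a track along a Spline component.
; Its Construction Script divides the spline length into fixed-spacing segments, taking each local transform with an added 90-degree yaw.
; Each segment gets two side-by-side child actors and a scaled, shadowless static mesh, positioned by composing offsets onto that transform.
; The event graph is empty, so the Blueprint adds no runtime logic.
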(event EventBeginPlay)

(event Collision|EventActorBeginOverlap
  (params (OtherActor :type Actor%20Object%20Reference)))

(event EventTick
  (params (DeltaSeconds :type Float%20%28single-precision%29)))

(fn ConstructionScript
  (bind _spline (Variables|Default|GetSpline))
  (for _index (range 0 (Math|Conversions|ToInteger(Byte) (- (Class|KismetMathLibrary|FFloor64 (/ (Spline|GetSplineLength _spline) 152.0)) 1)))
    (AddComponent|AddChildActorComponent false (Math|Transform|MakeTransform (.Location (Math|Transform|BreakTransform (Spline|GetTransformatDistanceAlongSpline _spline (Math|Conversions|ToFloat(Integer) (+ (* _index 152) 50)) "Local" false))) (Math|Rotator|CombineRotators (Math|Rotator|MakeRotator 0.0 0.0 9e+01) (.Rotation (Math|Transform|BreakTransform (Spline|GetTransformatDistanceAlongSpline _spline (Math|Conversions|ToFloat(Integer) (+ (* _index 152) 50)) "Local" false)))) (.Scale (Math|Transform|BreakTransform (Spline|GetTransformatDistanceAlongSpline _spline (Math|Conversions|ToFloat(Integer) (+ (* _index 152) 50)) "Local" false)))))
    (AddComponent|AddChildActorComponent false (Math|Transform|ComposeTransforms (Math|Transform|MakeTransform "-152.000000,0.000000,0.000000") (Math|Transform|MakeTransform (.Location (Math|Transform|BreakTransform (Spline|GetTransformatDistanceAlongSpline _spline (Math|Conversions|ToFloat(Integer) (+ (* _index 152) 50)) "Local" false))) (Math|Rotator|CombineRotators (Math|Rotator|MakeRotator 0.0 0.0 9e+01) (.Rotation (Math|Transform|BreakTransform (Spline|GetTransformatDistanceAlongSpline _spline (Math|Conversions|ToFloat(Integer) (+ (* _index 152) 50)) "Local" false)))) (.Scale (Math|Transform|BreakTransform (Spline|GetTransformatDistanceAlongSpline _spline (Math|Conversions|ToFloat(Integer) (+ (* _index 152) 50)) "Local" false))))))
    (bind _returnvalue (AddComponent|AddStaticMeshComponent false (Math|Transform|ComposeTransforms (Math|Transform|MakeTransform "-160.000000,0.000000,76.000000" "0, 0, 0" "1.537997,1.537997,1.537997") (Math|Transform|ComposeTransforms (Math|Transform|MakeTransform "-152.000000,0.000000,0.000000") (Math|Transform|MakeTransform (.Location (Math|Transform|BreakTransform (Spline|GetTransformatDistanceAlongSpline _spline (Math|Conversions|ToFloat(Integer) (+ (* _index 152) 50)) "Local" false))) (Math|Rotator|CombineRotators (Math|Rotator|MakeRotator 0.0 0.0 9e+01) (.Rotation (Math|Transform|BreakTransform (Spline|GetTransformatDistanceAlongSpline _spline (Math|Conversions|ToFloat(Integer) (+ (* _index 152) 50)) "Local" false)))) (.Scale (Math|Transform|BreakTransform (Spline|GetTransformatDistanceAlongSpline _spline (Math|Conversions|ToFloat(Integer) (+ (* _index 152) 50)) "Local" false))))))))
    (Rendering|SetCastShadow _returnvalue false)))