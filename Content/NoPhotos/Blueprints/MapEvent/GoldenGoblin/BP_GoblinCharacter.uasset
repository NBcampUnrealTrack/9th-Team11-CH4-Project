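; Golden goblin map-event character that laughs while idle and reacts to being photographed.
; On the server, a looping timer rolls a random chance during active gameplay to multicast a laugh at its location.
; Being photographed launches it upward, then plays an out sound if its photo HP is depleted, otherwise surprise and coin sounds.
; The photo-sound multicast is an empty stub, so those sounds play directly in the photographed event.
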(event Custom|Multicast_PlayPhotoSound)

(event Custom|TryPlayIdleSound
  (if (Class|NPGoblinCharacter|IsGameplayActive)
    (if (Math|Random|RandomBoolwithWeight 0.5)
      (CallFunction|MulticastPlayIdleSound))))

(event Custom|Multicast_PlayIdleSound
  (Audio|SpawnSoundatLocation "/Game/NoPhotos/Resources/Sound/SFX/MapEvent/Goblin/S_GoblinLaugh.S_GoblinLaugh" (Transformation|GetActorLocation) "0, 0, 0" 1.0 1.0 0.0 0 0))

(event EventBeginPlay
  (Networking|SwitchHasAuthority
    (:Authority
      (Utilities|Time|SetTimerbyEvent (delegate Custom|TryPlayIdleSound) 5.0 true))))

(event EventOnPhotographed
  (params (Photographer :type Player%20State%20Object%20Reference) (Visibility :type Float%20%28single-precision%29) (CaptureSequence :type Integer))
  (bind _returnvalue (Transformation|GetActorLocation))
  (Utilities|FlowControl|Sequence
    (:then_0
      (Character|LaunchCharacter "0.000000,0.000000,450.000000" false true))
    (:then_1
      (if (<= (Class|NPGoblinCharacter|GetCurrentPhotoHP) 0)
        (Audio|PlaySoundatLocation "/Game/NoPhotos/Resources/Sound/SFX/MapEvent/Goblin/S_GoblinOut.S_GoblinOut" _returnvalue "0, 0, 0" 1.0 1.0 0.0 "/Game/NoPhotos/Blueprints/MapEvent/GoldenGoblin/ATT_GoblinSound.ATT_GoblinSound" 0 0 0)
        (else
          (Audio|SpawnSoundatLocation "/Game/NoPhotos/Resources/Sound/SFX/MapEvent/Goblin/Goblin_Surprise1.Goblin_Surprise1" _returnvalue "0, 0, 0" 1.0 1.0 0.0 "/Game/NoPhotos/Blueprints/MapEvent/GoldenGoblin/ATT_GoblinSound.ATT_GoblinSound" 0)
          (Audio|SpawnSoundatLocation "/Game/NoPhotos/Resources/Sound/SFX/MapEvent/Coin.Coin" _returnvalue "0, 0, 0" 1.0 1.0 0.0 "/Game/NoPhotos/Blueprints/MapEvent/GoldenGoblin/ATT_GoblinSound.ATT_GoblinSound" 0))))))

(fn ConstructionScript)