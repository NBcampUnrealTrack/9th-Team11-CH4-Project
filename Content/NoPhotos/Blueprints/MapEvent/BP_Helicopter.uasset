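; BP_Helicopter is a map event actor that plays a portal effect and a light beam when it begins play.
; One timeline drives the Niagara system's User.EmitterScale parameter for the portal, while another animates the relative scale of the light beam component.
; The construction script gives the beam a dynamic material instance tinted purple.
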(event EventBeginPlay
  (Utilities|FlowControl|Sequence
    (:then_0
      (Components|Activation|Activate (Variables|Default|GetNiagara) false)
      (bind _newtrack_0 (Timeline|TL_Portal PlayFromStart)
        (:Update
          (Niagara|SetNiagaraVariable(Float) (Variables|Default|GetNiagara) "User.EmitterScale" _newtrack_0))))
    (:then_1
      (Components|Activation|Activate (Variables|Default|GetS_EV_SimpleLightBeam_01) false)
      (bind _newtrack_0_2 (Timeline|TL_LightBeam PlayFromStart)
        (:Update
          (Transformation|SetRelativeScale3D (Variables|Default|GetS_EV_SimpleLightBeam_01) _newtrack_0_2))))))

(fn ConstructionScript
  (bind _returnvalue (Rendering|Material|CreateDynamicMaterialInstance (Variables|Default|GetS_EV_SimpleLightBeam_01) 0 0 "None" :!class /Script/Engine.PrimitiveComponent))
  (Rendering|Material|SetVectorParameterValue _returnvalue "Color" "(R=0.257390,G=0.000000,B=0.427083,A=1.000000)" :!class /Script/Engine.MaterialInstanceDynamic))