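; Map event actor for the possession event, which applies a screen effect while the event is active.
; On BeginPlay it binds to the event-started delegate and plays a 2D ghost sound when the event starts.
; ApplyEventState calls the parent, then runs a fade-in or fade-out timeline that drives the possession post process's blend weight.
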(event Custom|OnEventStarted_Event
  (params (MapEvent :type NP%20Map%20Event%20Object%20Reference))
  (Audio|PlaySound2D "/Game/NoPhotos/Resources/Sound/SFX/MapEvent/Ghost/S_GhostEvent.S_GhostEvent" 1.0 1.0 0.0 0 0))

(event EventBeginPlay
  (EventDispatchers|AssignOnEventStarted (delegate Custom|OnEventStarted_Event)))

(event Collision|EventActorBeginOverlap
  (params (OtherActor :type Actor%20Object%20Reference)))

(event EventTick
  (params (DeltaSeconds :type Float%20%28single-precision%29)))

(event EventApplyEventState
  (params (bNewActive :type Boolean))
  (bind _possessionpostprocess (Variables|Default|GetPossessionPostProcess))
  (|CallParentFunction bNewActive)
  (if bNewActive
    (bind _newtrack_0 (Timeline|Fog_FadeIn PlayFromStart)
      (:Update
        (Variables|/Script/Engine.PostProcessComponent|SetBlendWeight _possessionpostprocess _newtrack_0)))
    (else
      (bind _newtrack_0_2 (Timeline|Fog_FadeOut PlayFromStart)
        (:Update
          (Variables|/Script/Engine.PostProcessComponent|SetBlendWeight _possessionpostprocess _newtrack_0_2))))))

(fn ConstructionScript)