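; Relic return zone actor for a map event, handling the visuals for delivered relics and the zone's appearance and departure.
; On delivery it spawns a BP_RelicReturnVisual from the relic's static mesh, which is sent straight up from the delivery location.
; Timelines on BeginPlay and bonus departure drive the jump pad Niagara effect's horizontal scale and its EmitterScale parameter together.
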(event EventBeginPlay
  (bind _ns_jumppad (Variables|Default|GetNS_JumpPad))
  (bind _newtrack_0 (Timeline|ScaleUp PlayFromStart)
    (:Update
      (Utilities|FlowControl|Sequence
        (:then_0
          (Transformation|SetRelativeScale3D _ns_jumppad (Math|Vector|MakeVector _newtrack_0 _newtrack_0 1.0)))
        (:then_1
          (Niagara|SetNiagaraVariable(Float) _ns_jumppad "User.EmitterScale" _newtrack_0))))))

(event EventBeginRelicBonusDeparture
  (params (DepartureDuration :type Float%20%28single-precision%29))
  (bind _ns_jumppad (Variables|Default|GetNS_JumpPad))
  (bind _newtrack_0 (Timeline|Timeline PlayFromStart)
    (:Update
      (Utilities|FlowControl|Sequence
        (:then_0
          (Transformation|SetRelativeScale3D _ns_jumppad (Math|Vector|MakeVector _newtrack_0 _newtrack_0 1.0)))
        (:then_1
          (Niagara|SetNiagaraVariable(Float) _ns_jumppad "User.EmitterScale" _newtrack_0))))))

(event EventTick
  (params (DeltaSeconds :type Float%20%28single-precision%29)))

(event EventOnRelicDelivered
  (params (DeliveredRelic :type NP%20Base%20Relic%20Object%20Reference) (DeliveryLocation :type Vector :default "0, 0, 0"))
  (bind _returnvalue (Class|NPBaseRelic|GetRelicMeshComponent DeliveredRelic))
  (Utilities|IsValid _returnvalue
    (:Is%20Valid
      (bind _asstatic_mesh_component (Utilities|Casting|CastToStaticMeshComponent _returnvalue))
      (bind _returnvalue_2 (Game|SpawnActorfromClass "/Game/NoPhotos/Blueprints/MapEvent/RelicReturnBonus/BP_RelicReturnVisual.BP_RelicReturnVisual_C" (Math|Transform|MakeTransform DeliveryLocation "0, 0, 0" "1.000000,1.000000,1.000000") "Undefined" "MultiplyWithRoot" 0 0))
      (Default|InitializeReturnVisual _returnvalue_2 _asstatic_mesh_component DeliveryLocation (+ DeliveryLocation "0.000000,0.000000,2000.000000") 2.0))))

(event Collision|EventActorBeginOverlap
  (params (OtherActor :type Actor%20Object%20Reference)))

(fn ConstructionScript)