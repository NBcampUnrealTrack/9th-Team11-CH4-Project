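; BP_Helicopter is a relic return bonus map event actor that shows a purple portal effect, despite its helicopter name.
; On BeginPlay, parallel timelines drive the Niagara emitter scale and the light beam and sphere mesh scales, alongside a 2D portal-open sound.
; BeginRelicBonusDeparture runs separate timelines on the same components for the departure effect.
; The construction script tints beam and sphere through dynamic materials; GetHeldRelic is an empty stub.
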(event EventBeginPlay
  (Utilities|FlowControl|Sequence
    (:then_0
      (Components|Activation|Activate (Variables|Default|GetNiagara) false)
      (bind _newtrack_0 (Timeline|TL_Portal PlayFromStart)
        (:Update
          (Niagara|SetNiagaraVariable(Float) (Variables|Default|GetNiagara) "User.EmitterScale" _newtrack_0))))
    (:then_1
      (Components|Activation|Activate (Variables|Default|GetS_EV_SimpleLightBeam_01) false)
      (bind _newtrack_0_2 (Timeline|TL_LightBeam PlayFromStart)
        (:Update
          (Transformation|SetRelativeScale3D (Variables|Default|GetS_EV_SimpleLightBeam_01) _newtrack_0_2))))
    (:then_2
      (Audio|PlaySound2D "/Game/NoPhotos/Resources/Sound/SFX/MapEvent/BonusRelic/S_PortalOpen.S_PortalOpen" 1.0 1.0 0.0 0 0))
    (:then_3
      (Components|Activation|Activate (Variables|Default|GetSphere) false)
      (bind _newtrack_0_3 (Timeline|Timeline_1 PlayFromStart)
        (:Update
          (Transformation|SetRelativeScale3D (Variables|Default|GetSphere) _newtrack_0_3))))))

(event EventBeginRelicBonusDeparture
  (params (DepartureDuration :type Float%20%28single-precision%29))
  (Utilities|FlowControl|Sequence
    (:then_0
      (Components|Activation|Activate (Variables|Default|GetNiagara) false)
      (bind _newtrack_0 (Timeline|Timeline PlayFromStart)
        (:Update
          (Niagara|SetNiagaraVariable(Float) (Variables|Default|GetNiagara) "User.EmitterScale" _newtrack_0))))
    (:then_1
      (Components|Activation|Activate (Variables|Default|GetS_EV_SimpleLightBeam_01) false)
      (bind _newtrack_0_2 (Timeline|Timeline_0 PlayFromStart)
        (:Update
          (Transformation|SetRelativeScale3D (Variables|Default|GetS_EV_SimpleLightBeam_01) _newtrack_0_2))))
    (:then_2
      (bind _newtrack_0_3 (Timeline|Timeline_2 PlayFromStart)
        (:Update
          (Transformation|SetRelativeScale3D (Variables|Default|GetSphere) _newtrack_0_3))))))

(fn ConstructionScript
  (Utilities|FlowControl|Sequence
    (:then_0
      (bind _returnvalue (Rendering|Material|CreateDynamicMaterialInstance (Variables|Default|GetSphere) 0 0 "None" :!class /Script/Engine.PrimitiveComponent))
      (Rendering|Material|SetVectorParameterValue _returnvalue "PInt" "(R=0.257390,G=0.000000,B=0.427083,A=1.000000)" :!class /Script/Engine.MaterialInstanceDynamic))
    (:then_1
      (bind _returnvalue_2 (Rendering|Material|CreateDynamicMaterialInstance (Variables|Default|GetS_EV_SimpleLightBeam_01) 0 0 "None" :!class /Script/Engine.PrimitiveComponent))
      (Rendering|Material|SetVectorParameterValue _returnvalue_2 "Color" "(R=0.257390,G=0.000000,B=0.427083,A=1.000000)" :!class /Script/Engine.MaterialInstanceDynamic))))

(fn GetHeldRelic
  (return 0))