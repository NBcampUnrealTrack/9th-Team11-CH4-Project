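; Hot potato bomb actor for a map event, handling the bomb's countdown visuals, audio and explosion effects.
; A timeline pulses mesh scale and triggers tick sounds, with Tick raising its play rate in steps as remaining fuse time drops.
; A dynamic material tints from black to red over the final seconds, alongside a one-shot time-limit warning sound.
; OnBombExploded stops the pulse and ticking, then spawns Niagara and sound effects.
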(event EventBeginPlay
  (Utilities|FlowControl|Sequence
    (:then_0
      (bind _output_get (Variables|Default|SetBaseBombScale (Variables|/Script/Engine.SceneComponent|GetRelativeScale3D (Variables|Default|GetBombMesh))))
      (bind _newtrack_2 (Timeline|Timeline PlayFromStart)
        (:Update
          (Transformation|SetRelativeScale3D (Variables|Default|GetBombMesh) (* _output_get _newtrack_2)))
        (:NewTrack_0
          (Audio|Components|Audio|Play (Variables|Default|GetBombTickAudio) 0.0))))
    (:then_1
      (bind _returnvalue (Rendering|Material|CreateDynamicMaterialInstance (Variables|Default|GetBombMesh) 0 "/Game/NoPhotos/Blueprints/MapEvent/HotPotato/M_Bomb.M_Bomb" "None" :!class /Script/Engine.PrimitiveComponent))
      (Variables|Default|SetBombMID _returnvalue))))

(event EventTick
  (params (DeltaSeconds :type Float%20%28single-precision%29))
  (bind _returnvalue (Class|NPHotPotatoBomb|GetRemainingFuseTime))
  (bind _timeline (Variables|Default|GetTimeline))
  (Utilities|FlowControl|Sequence
    (:then_0
      (if (<= _returnvalue 2.0)
        (Components|Timeline|SetPlayRate _timeline 4.0)
        (elif (<= _returnvalue 5.0)
          (Components|Timeline|SetPlayRate _timeline 3.0)
          (Utilities|FlowControl|DoOnce false
            (:Completed
              (Audio|SpawnSoundAttached "/Game/NoPhotos/Resources/Sound/SFX/MapEvent/HotPotato/S_TimeLimit.S_TimeLimit" (Variables|Default|GetBombMesh) "None" "0, 0, 0" "0, 0, 0" "KeepRelativeOffset" true 0.5 0.8 0.0 0 0)))
          (elif (<= _returnvalue 1e+01)
            (Components|Timeline|SetPlayRate _timeline 2.0)
            (else
              (Components|Timeline|SetPlayRate _timeline 1.0))))))
    (:then_1
      (Rendering|Material|SetVectorParameterValue (Variables|Default|GetBombMID) "BombTint" (Math|Color|Lerp(LinearColor) (Utilities|Struct|MakeLinearColor 0.0 0.0 0.0 1.0) (Utilities|Struct|MakeLinearColor 1.0 0.0 0.0 1.0) (Math|Float|MapRangeClamped (Class|NPHotPotatoBomb|GetRemainingFuseTime) 1e+01 0.0 0.0 1.0)) :!class /Script/Engine.MaterialInstanceDynamic))))

(event EventOnBombExploded
  (params (ExplosionLocation :type Vector :default "0, 0, 0"))
  (bind _returnvalue (Transformation|GetActorLocation))
  (Utilities|FlowControl|Sequence
    (:then_0
      (Audio|Components|Audio|Stop (Variables|Default|GetTimeline)))
    (:then_1
      (Audio|Components|Audio|Stop (Variables|Default|GetBombTickAudio)))
    (:then_2
      (Niagara|SpawnSystematLocation "/Game/Fire_EXP_Vol01_Free/Niagara/EXP/NS_Sub_EXP_Large_001_01.NS_Sub_EXP_Large_001_01" _returnvalue)
      (Audio|SpawnSoundatLocation "/Game/NoPhotos/Resources/Sound/SFX/Relic/soundreality-explosion-fx-343683.soundreality-explosion-fx-343683" _returnvalue "0, 0, 0" 0.5 1.0 0.0 "/Game/NoPhotos/Blueprints/Relic/GeometryCollections/ATT_Nearby.ATT_Nearby" 0))))

(fn ConstructionScript)

(fn NewFunction)

(fn NewFunction0)