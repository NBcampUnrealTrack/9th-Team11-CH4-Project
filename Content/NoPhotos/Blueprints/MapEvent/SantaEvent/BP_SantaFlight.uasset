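; BP_SantaFlight is the flying Santa actor for the Santa map event, providing its wind effect and audio.
; On BeginPlay it spawns an unattached, hugely scaled ground-wind Niagara system and attaches bell and boosted laugh sounds to FlightRoot, set to stop when it is destroyed.
; EndPlay destroys the stored particle component; the event graph contains no movement logic.
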(event Collision|EventActorBeginOverlap
  (params (OtherActor :type Actor%20Object%20Reference)))

(event EventTick
  (params (DeltaSeconds :type Float%20%28single-precision%29)))

(event EventBeginPlay
  (bind _returnvalue (Transformation|GetActorLocation))
  (bind _flightroot (Variables|Default|GetFlightRoot))
  (if true
    (bind _returnvalue_2 (Niagara|SpawnSystematLocation "/Game/NoPhotos/Blueprints/MapEvent/NS_RelicBonus_GroundWind.NS_RelicBonus_GroundWind" "0, 0, 0"))
    (bind _output_get (Variables|Default|Setparticle _returnvalue_2))
    (Transformation|SetRelativeScale3D _output_get "100.000000,100.000000,100.000000")
    (Audio|SpawnSoundAttached "/Game/NoPhotos/Resources/Sound/SFX/MapEvent/Santa/S_Bell.S_Bell" _flightroot "None" _returnvalue "0, 0, 0" "KeepRelativeOffset" true 1.0 1.0 0.0 0 0)
    (Audio|SpawnSoundAttached "/Game/NoPhotos/Resources/Sound/SFX/MapEvent/Santa/S_SantaLaugh.S_SantaLaugh" _flightroot "None" _returnvalue "0, 0, 0" "KeepRelativeOffset" true 6.0 1.0 0.0 0 0)))

(event EventEndPlay
  (params (EndPlayReason :type EEndPlayReason%20Enum :default "Destroyed"))
  (bind _particle (Variables|Default|Getparticle))
  (Utilities|IsValid _particle
    (:Is%20Valid
      (Components|DestroyComponent _particle))))

(fn ConstructionScript)